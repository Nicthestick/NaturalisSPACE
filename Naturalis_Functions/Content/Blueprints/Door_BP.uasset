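; Proximity-triggered three-panel door that opens when the player enters its trigger while unlocked and closes after they leave.
; Separate open and close timelines lerp the panels between start and end positions, with audio for each and a particle burst after closing.
; DoorOpen and DoorMoving flags gate transitions, with 0.2-second Delay loops polling door state.
; A similar loop from BeginPlay colors two lights red or green from DoorLocked.
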(event `self.ReceiveBeginPlay`
  (bind _light1 (`self.light1`))
  (bind _light1_2 (`self.light1`))
  (bind _light2 (`self.light2`))
  (bind _light2_2 (`self.light2`))
  (set `self.PlayerInTrigger` false)
  (set `self.DoorOpen` false)
  (set `self.DoorMoving` false)
  (if (`self.DoorLocked`) :!label _label
    (`/Engine/EditorBlueprintResources/StandardMacros.IsValid` _light1_2
      (:`Is Valid`
        (`PrimitiveComponent.SetMaterial` _light1_2 0 "/Game/Materials/M_Light_Red.M_Light_Red")
        (`/Engine/EditorBlueprintResources/StandardMacros.IsValid` _light2
          (:`Is Valid`
            (`PrimitiveComponent.SetMaterial` _light2 0 "/Game/Materials/M_Light_Red.M_Light_Red")))))
    (else
      (`/Engine/EditorBlueprintResources/StandardMacros.IsValid` _light1
        (:`Is Valid`
          (`PrimitiveComponent.SetMaterial` _light1 0 "/Game/Materials/M_Light_Green.M_Light_Green")
          (`/Engine/EditorBlueprintResources/StandardMacros.IsValid` _light2_2
            (:`Is Valid`
              (`PrimitiveComponent.SetMaterial` _light2_2 0 "/Game/Materials/M_Light_Green.M_Light_Green")))))))
  (`KismetSystemLibrary.Delay` 0.2)
  (goto _label))

(event `self.Trigger.OnComponentBeginOverlap`
  (params (OverlappedComponent :type "PrimitiveComponent Object Reference") (OtherActor :type "Actor Object Reference") (OtherComp :type "PrimitiveComponent Object Reference") (OtherBodyIndex :type Integer) (bFromSweep :type Boolean) (SweepResult :type "HitResult Structure (by ref)"))
  (set `self.PlayerInTrigger` true)
  (if (not (`self.DoorLocked`))
    (if (`self.DoorOpen`) :!label _label_2
      (`KismetSystemLibrary.Delay` 0.2)
      (if (`self.PlayerInTrigger`)
        (goto _label_2))
      (elif (not (`self.DoorMoving`))
        (set `self.DoorMoving` true)
        (`AudioComponent.Play` (`self.DoorAudio_OPEN`) 0.0)
        (bind (_direction _driver) (`Timeline|DoorTimerOpen` :!via `PlayFromStart`)
          (:`Update`
            (`SceneComponent.K2_SetRelativeLocation` (`self.Door1_H`) (`KismetMathLibrary.VLerp` (`self.Door1Start`) (`self.Door1End`) _driver) false false)
            (`SceneComponent.K2_SetRelativeLocation` (`self.Door2_H`) (`KismetMathLibrary.VLerp` (`self.Door2Start`) (`self.Door2End`) _driver) false false)
            (`SceneComponent.K2_SetRelativeLocation` (`self.Door3_V`) (`KismetMathLibrary.VLerp` (`self.Door3Start`) (`self.Door3End`) _driver) false false)
            (`KismetSystemLibrary.Delay` 2.0)
            (set `self.DoorOpen` true)
            (set `self.DoorMoving` false)))))))

(event `self.Trigger.OnComponentEndOverlap`
  (params (OverlappedComponent :type "PrimitiveComponent Object Reference") (OtherActor :type "Actor Object Reference") (OtherComp :type "PrimitiveComponent Object Reference") (OtherBodyIndex :type Integer))
  (set `self.PlayerInTrigger` false)
  (if (`self.DoorOpen`) :!label _label_3
    (if (not (`self.DoorMoving`))
      (set `self.DoorMoving` true)
      (`AudioComponent.Play` (`self.DoorAudio_CLOSE`) 0.0)
      (bind (_direction _driver) (`Timeline|DoorTimerClose` :!via `ReverseFromEnd`)
        (:`Update`
          (`SceneComponent.K2_SetRelativeLocation` (`self.Door1_H`) (`KismetMathLibrary.VLerp` (`self.Door1Start`) (`self.Door1End`) _driver) false false)
          (`SceneComponent.K2_SetRelativeLocation` (`self.Door2_H`) (`KismetMathLibrary.VLerp` (`self.Door2Start`) (`self.Door2End`) _driver) false false)
          (`SceneComponent.K2_SetRelativeLocation` (`self.Door3_V`) (`KismetMathLibrary.VLerp` (`self.Door3Start`) (`self.Door3End`) _driver) false false))
        (:`Finished`
          (`ActorComponent.Activate` (`self.ParticleSystem`) true)
          (`ActorComponent.Activate` (`self.ParticleSystem1`) true)
          (`ActorComponent.Activate` (`self.ParticleSystem2`) true)
          (`ActorComponent.Activate` (`self.ParticleSystem3`) true)
          (`KismetSystemLibrary.Delay` 2.0)
          (`ActorComponent.Deactivate` (`self.ParticleSystem`))
          (`ActorComponent.Deactivate` (`self.ParticleSystem1`))
          (`ActorComponent.Deactivate` (`self.ParticleSystem2`))
          (`ActorComponent.Deactivate` (`self.ParticleSystem3`))
          (`KismetSystemLibrary.Delay` 0.5)
          (set `self.DoorOpen` false)
          (set `self.DoorMoving` false))))
    (else
      (`KismetSystemLibrary.Delay` 0.2)
      (if (not (`self.PlayerInTrigger`))
        (goto _label_3)))))

(fn `UserConstructionScript`)