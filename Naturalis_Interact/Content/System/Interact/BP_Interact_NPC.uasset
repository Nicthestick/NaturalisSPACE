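; Interactable NPC that shows a three-page, image-based talk sequence on screen, building on its parent's interaction events.
; The first Interact creates an NPCWidget showing page one; later presses step through a looping MultiGate to show the next images, then close it.
; The interact prompt changes between Talk, Next and Close.
; Removing interactions also closes the widget and resets the prompt, but leaves the MultiGate's position as is.
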(event `self.ReceiveBeginPlay`
  (`parent.ReceiveBeginPlay`)
  (set `self.Interacted` false))

(event `self.ReceiveTick`
  (params (DeltaSeconds :type "Float (single-precision)")))

(event `self.removeInteractions`
  (params (Object :type "Object Object Reference"))
  (`parent.removeInteractions` Object)
  (`Widget.RemoveFromParent` (stale _returnvalue) :!label _label)
  (set `self.Interacted` false)
  (set `self.uiDescription` "Talk")
  (bind _asbp_interact_ui (cast `/Game/System/Interact/BP_Interact_UI` (`WidgetComponent.GetUserWidgetObject` (`self.interactUI`))))
  (`/Game/System/Interact/BP_Interact_UI.SetInteractDescription` _asbp_interact_ui (`self.uiDescription`)))

(event `self.interact`
  (params (interactCharacter :type "/Game/System/Interact/ThirdPersonCharacter_Interact Object Reference"))
  (`parent.interact` interactCharacter)
  (if (`self.Interacted`)
    (`|MultiGate` false true
      (:`Out 0`
        (bind _asnpcwidget (cast `/Game/System/NPC/NPC_HUD/NPCWidget` (stale _returnvalue)))
        (`/Game/System/NPC/NPC_HUD/NPCWidget.TurnOffImage1` _asnpcwidget)
        (`/Game/System/NPC/NPC_HUD/NPCWidget.TurnOffImage3` _asnpcwidget)
        (`/Game/System/NPC/NPC_HUD/NPCWidget.TurnOnImage2` _asnpcwidget))
      (:`Out 1`
        (bind _asnpcwidget_2 (cast `/Game/System/NPC/NPC_HUD/NPCWidget` (stale _returnvalue)))
        (`/Game/System/NPC/NPC_HUD/NPCWidget.TurnOffImage1` _asnpcwidget_2)
        (`/Game/System/NPC/NPC_HUD/NPCWidget.TurnOffImage2` _asnpcwidget_2)
        (`/Game/System/NPC/NPC_HUD/NPCWidget.TurnOnImage3` _asnpcwidget_2)
        (set `self.uiDescription` "Close")
        (bind _asbp_interact_ui (cast `/Game/System/Interact/BP_Interact_UI` (`WidgetComponent.GetUserWidgetObject` (`self.interactUI`))))
        (`/Game/System/Interact/BP_Interact_UI.SetInteractDescription` _asbp_interact_ui (`self.uiDescription`)))
      (:`Out 2`
        (bind _asnpcwidget_3 (cast `/Game/System/NPC/NPC_HUD/NPCWidget` (stale _returnvalue)))
        (`/Game/System/NPC/NPC_HUD/NPCWidget.TurnOffImage1` _asnpcwidget_3)
        (`/Game/System/NPC/NPC_HUD/NPCWidget.TurnOffImage2` _asnpcwidget_3)
        (`/Game/System/NPC/NPC_HUD/NPCWidget.TurnOffImage3` _asnpcwidget_3)
        (goto _label)))
    (else
      (bind _returnvalue (`|CreateWidget` "/Game/System/NPC/NPC_HUD/NPCWidget.NPCWidget_C"))
      (bind _asnpcwidget_4 (cast `/Game/System/NPC/NPC_HUD/NPCWidget` _returnvalue))
      (`/Game/System/NPC/NPC_HUD/NPCWidget.TurnOffImage2` _asnpcwidget_4)
      (`/Game/System/NPC/NPC_HUD/NPCWidget.TurnOffImage3` _asnpcwidget_4)
      (`/Game/System/NPC/NPC_HUD/NPCWidget.TurnOnImage1` _asnpcwidget_4)
      (`UserWidget.AddToViewport` _returnvalue 0)
      (set `self.Interacted` true)
      (set `self.uiDescription` "Next")
      (bind _asbp_interact_ui_2 (cast `/Game/System/Interact/BP_Interact_UI` (`WidgetComponent.GetUserWidgetObject` (`self.interactUI`))))
      (`/Game/System/Interact/BP_Interact_UI.SetInteractDescription` _asbp_interact_ui_2 (`self.uiDescription`)))))

(fn `UserConstructionScript`
  (`parent.UserConstructionScript`))