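; Base interactable actor that a ThirdPersonCharacter_Interact can register with and interact with.
; The construction script applies configurable mesh, trigger sphere and UI widget settings, and BeginPlay passes the description text to the BP_Interact_UI widget.
; Trigger overlaps add or remove the actor from the character's interactions.
; ToggleUI shows or hides the prompt, while Interact stores the character and prints a placeholder message.
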(event `self.ReceiveBeginPlay`
  (bind _asbp_interact_ui (cast `/Game/System/Interact/BP_Interact_UI` (`WidgetComponent.GetUserWidgetObject` (`self.interactUI`))))
  (`/Game/System/Interact/BP_Interact_UI.SetInteractDescription` _asbp_interact_ui (`self.uiDescription`)))

(event `self.interactTrigger.OnComponentBeginOverlap`
  (params (OverlappedComponent :type "PrimitiveComponent Object Reference") (OtherActor :type "Actor Object Reference") (OtherComp :type "PrimitiveComponent Object Reference") (OtherBodyIndex :type Integer) (bFromSweep :type Boolean) (SweepResult :type "HitResult Structure (by ref)"))
  (`self.addInteractions` OtherActor))

(event `self.interactTrigger.OnComponentEndOverlap`
  (params (OverlappedComponent :type "PrimitiveComponent Object Reference") (OtherActor :type "Actor Object Reference") (OtherComp :type "PrimitiveComponent Object Reference") (OtherBodyIndex :type Integer))
  (`self.removeInteractions` OtherActor))

(fn `addInteractions`
  (params (Object :type "Object Object Reference"))
  (bind _asthird_person_character_interact (cast `/Game/System/Interact/ThirdPersonCharacter_Interact` Object))
  (`/Game/System/Interact/ThirdPersonCharacter_Interact.AddInteraction` _asthird_person_character_interact self))

(fn `interact`
  (params (interactCharacter :type "/Game/System/Interact/ThirdPersonCharacter_Interact Object Reference"))
  (set `self.interactCharacter` interactCharacter)
  (`KismetSystemLibrary.PrintString` "INTERACTED"))

(fn `removeInteractions`
  (params (Object :type "Object Object Reference"))
  (bind _asthird_person_character_interact (cast `/Game/System/Interact/ThirdPersonCharacter_Interact` Object))
  (`/Game/System/Interact/ThirdPersonCharacter_Interact.RemoveInteraction` _asthird_person_character_interact self))

(fn `setupMesh`
  ;[1 1 1] Set Mesh Model and Transform
  (`StaticMeshComponent.SetStaticMesh` (`self.interactMesh`) (`self.meshModel`))
  (`SceneComponent.K2_SetRelativeTransform` (`self.interactMesh`) (`self.meshTransform`) false false))

(fn `setupTrigger`
  ;[1 1 1] Set the trigger size and location
  (`SphereComponent.SetSphereRadius` (`self.interactTrigger`) (`self.triggerRadius`) true)
  (`SceneComponent.K2_SetRelativeLocation` (`self.interactTrigger`) (`self.triggerLocation`) false false))

(fn `setupUI`
  ;[1 1 1] Set location offset for UI
  (`SceneComponent.K2_SetRelativeLocation` (`self.interactUI`) (`self.uiLocaton`) false false))

(fn `toggleUI`
  (params (b_Visible :type Boolean))
  ;[1 1 1] Set Visiblity of UI
  (`SceneComponent.SetVisibility` (`self.interactUI`) b_Visible false))

(fn `UserConstructionScript`
  (`self.setupMesh`)
  (`self.setupTrigger`)
  (`self.setupUI`))